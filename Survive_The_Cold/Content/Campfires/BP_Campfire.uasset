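; BP_Campfire is a campfire that restores the player's Warmth in the game instance and then becomes unusable.
; Overlapping its trigger as a Player-tagged actor shows a "press E" widget, removed on end overlap.
; IsEPressed is checked only at overlap start; if set, the sprite changes for a timed delay before reverting and disabling reuse.
; BeginPlay caches references, casting the overlap event's OtherActor for the character.
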(event OnComponentBeginOverlap(Trigger)
  (params (OverlappedComponent :type Primitive%20Component%20Object%20Reference) (OtherActor :type Actor%20Object%20Reference) (OtherComp :type Primitive%20Component%20Object%20Reference) (OtherBodyIndex :type Integer) (bFromSweep :type Boolean) (SweepResult :type Hit%20Result%20Structure%20%28by%20ref%29))
  (if (Actor|ActorHasTag OtherActor "Player")
    (UserInterface|Viewport|AddtoViewport (stale EventBeginPlay _returnvalue) 0)
    (if (Variables|/Game/Character/BP_TopDownChar.BP_TopDownChar_C|GetIsEPressed? (Variables|Default|GetBP%20Top%20Down%20Char%20Ref))
      (if (Variables|Default|GetCanUseCampfire?)
        (Rendering|Components|Sprite|SetSprite (Variables|Default|GetCampfire) "/Game/Campfires/traveler_s_camp_Sprite_24.traveler_s_camp_Sprite_24")
        (Variables|/Game/BP_GameInst.BP_GameInst_C|SetWarmth (Variables|Default|GetBP%20Game%20Inst%20Ref) 1e+02)
        (Utilities|FlowControl|Delay 15.0)
        (Rendering|Components|Sprite|SetSprite (Variables|Default|GetCampfire) "/Game/Campfires/traveler_s_camp_Sprite_4.traveler_s_camp_Sprite_4")
        (Variables|Default|SetCanUseCampfire? false)))))

(event OnComponentEndOverlap(Trigger)
  (params (OverlappedComponent :type Primitive%20Component%20Object%20Reference) (OtherActor :type Actor%20Object%20Reference) (OtherComp :type Primitive%20Component%20Object%20Reference) (OtherBodyIndex :type Integer))
  (Widget|RemovefromParent (stale EventBeginPlay _returnvalue)))

(event EventBeginPlay
  (bind _asbp_game_inst (Utilities|Casting|CastToBP_GameInst (Game|GetGameInstance)))
  (Variables|Default|SetBP%20Game%20Inst%20Ref _asbp_game_inst)
  (bind _returnvalue (UserInterface|CreateWidget "/Game/Campfires/PressEText.PressEText_C"))
  (bind _asbp_top_down_char (Utilities|Casting|CastToBP_TopDownChar (stale OnComponentBeginOverlap(Trigger) OtherActor)))
  (Variables|Default|SetBP%20Top%20Down%20Char%20Ref _asbp_top_down_char))

(fn ConstructionScript)