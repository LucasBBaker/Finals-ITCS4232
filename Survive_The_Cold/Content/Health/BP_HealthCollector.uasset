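; BP_HealthCollector is a pickup that restores a fixed amount of the player's health.
; On BeginPlay it caches the BP_GameInst game instance, which stores the Health value.
; When an actor tagged Player overlaps the Trigger component and Health is not exactly full, it adds health without clamping, plays a click sound at the world origin and destroys itself.
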(event OnComponentBeginOverlap(Trigger)
  (params (OverlappedComponent :type Primitive%20Component%20Object%20Reference) (OtherActor :type Actor%20Object%20Reference) (OtherComp :type Primitive%20Component%20Object%20Reference) (OtherBodyIndex :type Integer) (bFromSweep :type Boolean) (SweepResult :type Hit%20Result%20Structure%20%28by%20ref%29))
  (bind _bp_game_inst_ref (Variables|Default|GetBP%20Game%20Inst%20Ref))
  (if (Actor|ActorHasTag OtherActor "Player")
    (if (not (== (Variables|/Game/BP_GameInst.BP_GameInst_C|GetHealth (Variables|Default|GetBP%20Game%20Inst%20Ref)) 1e+02))
      (Variables|/Game/BP_GameInst.BP_GameInst_C|SetHealth _bp_game_inst_ref (+ (Variables|/Game/BP_GameInst.BP_GameInst_C|GetHealth _bp_game_inst_ref) 1e+01))
      (Audio|PlaySoundatLocation "/Engine/VREditor/Sounds/VR_click3.VR_click3" "0, 0, 0" "0, 0, 0" 1.0 1.0 0.0 0 0 0 0)
      (Actor|DestroyActor))))

(event EventBeginPlay
  (bind _asbp_game_inst (Utilities|Casting|CastToBP_GameInst (Game|GetGameInstance)))
  (Variables|Default|SetBP%20Game%20Inst%20Ref _asbp_game_inst))

(fn ConstructionScript)